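; AI controller for a child pawn (BP_child) that, judging by its name, runs away from perceived threats.
; On possess it runs BT_Child; sensing an actor tagged "target" cancels the forget timer and sets that actor on the blackboard and pawn.
; Any other perception update starts a short timer that clears the target and the scream flag.
; Perception is deactivated on unpossess.
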(event OnTargetPerceptionUpdated(AIPerception)
  (params (Actor :type Actor%20Object%20Reference) (Stimulus :type AI%20Stimulus%20Structure))
  (if (and (Actor|ActorHasTag Actor "target") (.bSuccessfullySensed (Utilities|Struct|BreakAIStimulus Stimulus)))
    (Utilities|Time|ClearandInvalidateTimerbyHandle (Variables|Default|GetEnemyTimer))
    (AI|Components|Blackboard|SetValueasObject (Variables|Default|GetBlackboard) (Variables|Default|GetBBTargetActor) Actor)
    (bind _asbp_child (Utilities|Casting|CastToBP_child (Variables|Default|GetPossessed%20Pawn)))
    (Default|SetTarget _asbp_child Actor)
    (else
      (bind _returnvalue (Utilities|Time|SetTimerbyEvent (delegate Custom|StartEnemyTimer) 4.0))
      (Variables|Default|SetEnemyTimer _returnvalue))))

(event Custom|StartEnemyTimer
  (AI|Components|Blackboard|SetValueasObject (Variables|Default|GetBlackboard) (Variables|Default|GetBBTargetActor) 0)
  (bind _asbp_child (Utilities|Casting|CastToBP_child (Variables|Default|GetPossessed%20Pawn)))
  (Default|SetTarget _asbp_child)
  (AI|Components|Blackboard|SetValueasBool (Variables|Default|GetBlackboard) (Variables|Default|GetBBShouldScream) false))

(event EventPossess
  (params (PossessedPawn :type Pawn%20Object%20Reference))
  (Variables|Default|SetPossessed%20Pawn PossessedPawn)
  (AI|RunBehaviorTree "/Game/Blueprints/Child/BT_Child.BT_Child"))

(event EventUnPossess
  (params (UnpossessedPawn :type Pawn%20Object%20Reference))
  (Components|Activation|SetActive (Variables|Default|GetAIPerception) false false))

(fn ConstructionScript)