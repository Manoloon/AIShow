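; Base Blueprint for an AI Kungfu Circle, which by its name and functions limits characters around a target through a weighted slot budget.
; SlotsWeight stores available weight in X and capacity in Y, with a setter clamped to that capacity and a reset that refills it.
; Register, Unregister, IsContains and GetCircleType are placeholders returning defaults.
; CalcPosition returns cosine and sine of Degrees multiplied by Radius, without scaling the result.
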(fn ConstructionScript)

(fn CalcPosition
  (params (degrees :type Float%20%28double-precision%29) (radius :type Float%20%28double-precision%29))
  (bind _returnvalue (* degrees radius))
  (return (Math|Vector|MakeVector (Math|Trig|Cos(Degrees) _returnvalue) (Math|Trig|Sin(Degrees) _returnvalue) 0.0)))

(fn GetAvailableSlotsWeight
  (return (.x (Variables|Settings|GetSlotsWeight))))

(fn GetCapacitySlotsWeight
  (return (.y (Variables|Settings|GetSlotsWeight))))

(fn SetAvailableSlotsWeight
  (params (weight :type Float%20%28double-precision%29))
  (Variables|Settings|SetSlotsWeight (Math|Vector2D|MakeVector2D (Math|Float|Clamp(Float) weight 0.0 (.y (Variables|Settings|GetSlotsWeight))) (.y (Variables|Settings|GetSlotsWeight)))))

(fn ResetAvailableSlotsWeight
  (Variables|Settings|SetSlotsWeight (Math|Vector2D|MakeVector2D (.y (Variables|Settings|GetSlotsWeight)) (.y (Variables|Settings|GetSlotsWeight)))))

(fn Register
  (params (Character :type Character%20Object%20Reference))
  (return false))

(fn Unregister
  (params (Character :type Character%20Object%20Reference))
  (return false))

(fn IsContains
  (params (Character :type Character%20Object%20Reference))
  (return false))

(fn GetCircleType
  (return "NewEnumerator0"))