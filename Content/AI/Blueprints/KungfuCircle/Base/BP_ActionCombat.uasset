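; BP_ActionCombat is a base combat action for the KungfuCircle AI, tracking an action's state and cooldown.
; Execute sets the running state and restarts a cooldown timer, which Tick advances until it reaches its limit and clears the cooldown flag.
; Stop and Idle set the other states independently of the cooldown, IsRunning and IsInThisState query the state, and Next is a stub returning false.
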(event EventBeginPlay
  (Variables|Default|SetMyself (Variables|Default|GetMyself))
  (Variables|Default|SetState "NewEnumerator0"))

(event EventTick
  (params (DeltaSeconds :type Float%20%28single-precision%29))
  (if (Variables|Settings|GetIsCooldown)
    (Variables|Settings|SetTimer (Math|Vector2D|MakeVector2D (+ (.x (Variables|Settings|GetTimer)) DeltaSeconds) (.y (Variables|Settings|GetTimer))))
    (if (>= (.x (Variables|Settings|GetTimer)) (.y (Variables|Settings|GetTimer)))
      (Variables|Settings|SetIsCooldown false))))

(fn ConstructionScript)

(fn Execute
  (Variables|Settings|SetTimer (Math|Vector2D|MakeVector2D 0.0 (.y (Variables|Settings|GetTimer))))
  (Variables|Settings|SetIsCooldown true)
  (Variables|Default|SetState "NewEnumerator1"))

(fn IsRunning
  (return (Utilities|Enum|Equal(Enum) (Variables|Default|GetState) "NewEnumerator1")))

(fn Stop
  (Variables|Default|SetState "NewEnumerator2"))

(fn Idle
  (Variables|Default|SetState "NewEnumerator0"))

(fn IsinThisState
  (params (ActionState :type E_ActionState%20Enum :default "NewEnumerator0"))
  (return (Utilities|Enum|Equal(Enum) ActionState (Variables|Default|GetState))))

(fn Next
  (return false))