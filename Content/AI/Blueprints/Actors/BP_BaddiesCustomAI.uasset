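; BP_BaddiesCustomAI is an enemy AI actor that walks toward an assigned target point.
; On BeginPlay, if Active is set, it calls its Move event.
; Move checks that TargetPoint is valid, then has its AI controller MoveToActor toward it using a configurable navigation filter class.
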(event Custom|Move
  (Utilities|IsValid (Variables|Default|GetTargetPoint)
    (:Is%20Valid
      (AI|Navigation|MovetoActor (AI|GetAIController self) (Variables|Default|GetTargetPoint) 5e+01 true true true (Variables|Default|GetFilter%20Class)))))

(event EventBeginPlay
  (if (Variables|Default|GetActive)
    (CallFunction|Move)))

(fn ConstructionScript)